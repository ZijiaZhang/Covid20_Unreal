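; Game mode that runs a people-based objective, declaring victory when the points tally matches the number of People spawned.
; SpawnPeople scatters People actors at random navigable points, randomly assigning a less common second type and counting only successful spawns.
; Addpoint increments the score and fires Victory on a match, showing a widget and restarting after a short delay.
; SpawnRocket places a player-owned GroundRocket at the pawn's location.
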(event Custom|Victory
  (bind _returnvalue (UserInterface|CreateWidget "/Game/UI/Victory.Victory_C"))
  (UserInterface|Viewport|AddtoViewport _returnvalue 0)
  (Utilities|FlowControl|Delay 2.0)
  (Class|GameMode|RestartGame))

(event EventBeginPlay)

(event EventTick
  (params (DeltaSeconds :type Float%20%28single-precision%29)))

(fn ConstructionScript)

(fn Addpoint
  (bind _points (Variables|Default|GetPoints))
  (Math|Integer|IncrementInt _points
    (:%20%20
      (if (== _points (Variables|Default|GetPeopleSpawned))
        (CallFunction|Victory)))))

(fn SpawnPeople
  (Variables|Default|SetPeopleSpawned 0)
  (for _index (range 0 (Variables|Default|GetPeopleCount))
    (bind _returnvalue (Game|SpawnActorfromClass "/Game/ThirdPersonBP/Blueprints/People.People_C" (Math|Conversions|ToTransform(Vector) (+ (.RandomLocation (Class|NavigationSystemV1|GetRandomPointinNavigableRadius (Math|Vector|MakeVector 0.0 0.0 0.0) 2e+03 0 0)) "0, 0,100.000000")) "AdjustIfPossibleButDontSpawnIfColliding" 0 (select (< (Math|Random|RandomFloat) 0.2) "NewEnumerator2" "NewEnumerator1") 0))
    (Utilities|IsValid _returnvalue
      (:Is%20Valid
        (Math|Integer|IncrementInt (Variables|Default|GetPeopleSpawned)
          (:%20%20
            (Development|PrintString "Hello")))))))

(fn SpawnRocket
  (bind _returnvalue (Game|Player|GetPlayerPawn 0))
  (Game|SpawnActorfromClass "/Game/ThirdPersonBP/Blueprints/GroundRocket.GroundRocket_C" (Math|Conversions|ToTransform(Vector) (Transformation|GetActorLocation _returnvalue)) "Undefined" _returnvalue 0))